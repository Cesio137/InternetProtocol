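; HTTP client Blueprint that lays out an HTTP client API as a node palette, with no live execution flow.
; Unconnected calls are grouped into Memory, Settings, Connection, Payload and Request, covering host setup, request building, sync or async payload preparation, processing and cancellation.
; Empty custom events match delegate bindings for payload, completion, progress, retry, error and cancel callbacks, but none of the bindings run.
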(event `AsyncPayloadFinished`
  ;[0 0 0] Events
)

(event `RequestCompleted` :!signature `self.OnRequestCompleted`
  (params (headers :type "Response Structure"))
  ;[0 0 0] Events
)

(event `RequestProgress` :!signature `self.OnRequestProgress`
  (params (bytesSent :type Integer) (bytesReceived :type Integer))
  ;[0 0 0] Events
)

(event `RequestWillRetry` :!signature `self.OnRequestWillRetry`
  (params (attemps :type Integer))
  ;[0 0 0] Events
)

(event `RequestError` :!signature `self.OnRequestError`
  (params (code :type Integer) (exception :type String))
  ;[0 0 0] Events
)

(event `ResponseError` :!signature `self.OnResponseError`
  (params (statusCode :type Integer))
  ;[0 0 0] Events
)

(event `RequestCanceled`
  ;[0 0 0] Events
)