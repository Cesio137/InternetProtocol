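; BPC_HttpClient is an HTTP client Blueprint that lays out the client API as an unwired catalogue, apparently as a reference or template.
; Loose nodes are grouped into socket, connection, payload, request and memory operations, alongside unused getters.
; Delegate bindings pair with empty custom events for payload preparation, progress, completion, response errors, closure and socket errors.
; Nothing executes: no call is connected and every handler is empty.
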(event `AsyncPayloadFinished`
  ;[0 0 0] Events
)

(event `RequestProgress` :!signature `self.OnRequestProgress`
  (params (BytesSent :type Integer) (BytesRecvd :type Integer))
  ;[0 0 0] Events
)

(event `RequestCompleted` :!signature `self.OnRequestCompleted`
  (params (Response :type "ClientResponse Structure"))
  ;[0 0 0] Events
)

(event `Response_Error` :!signature `self.OnResponseError`
  (params (Code :type Integer) (Message :type String))
  ;[0 0 0] Events
)

(event `ConnClose`
  ;[0 0 0] Events
)

(event `SocketError` :!signature `self.OnSocketError`
  (params (ErrorCode :type "ErrorCode Structure"))
  ;[0 0 0] Events
)

(event `Error` :!signature `self.OnError`
  (params (ErrorCode :type "ErrorCode Structure"))
  ;[0 0 0] Events
)