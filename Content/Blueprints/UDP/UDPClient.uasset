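; UDP client Blueprint laid out as an unwired reference of a socket API, with no executing logic.
; Loose, commented node groups cover remote host, connection, messaging and settings such as timeout, retry attempts, buffer sizes and packet splitting.
; Empty custom events pair with delegate bindings for connect, close, retry, send, receive and error, alongside unused status getters.
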(event `Connected`
  ;[0 0 0] Events
)

(event `ConnectionClose`
  ;[0 0 0] Events
)

(event `ConnectionWillRetry` :!signature `self.OnConnectionWillRetry`
  (params (attemp :type Integer))
  ;[0 0 0] Events
)

(event `MessageSent` :!signature `self.OnMessageSent`
  (params (size :type Integer))
  ;[0 0 0] Events
)

(event `MessageReceived` :!signature `self.OnMessageReceived`
  (params (size :type Integer) (message :type "UdpMessage Structure"))
  ;[0 0 0] Events
)

(event `Error` :!signature `self.OnError`
  (params (code :type Integer) (exception :type String))
  ;[0 0 0] Events
)