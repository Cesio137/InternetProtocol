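; BPC_UDPClient is a UDP client Blueprint component that lays out the socket API as an unwired node template.
; Groups cover host setup, connect and close, string and buffer sends, buffer-size and packet-split settings, and getters.
; Event stubs exist for connection, transfer, message, close and error delegates, but they are empty.
; No node chain, including the delegate bindings, is connected to an entry point, so none executes.
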(event `Connected`
  ;[0 0 0] Events
)

(event `BytesTransferred` :!signature `self.OnBytesTransferred`
  (params (BytesSent :type Integer) (BytesRecvd :type Integer))
  ;[0 0 0] Events
)

(event `MessageSent`
  ;[0 0 0] Events
)

(event `MessageReceived` :!signature `self.OnMessageReceived`
  (params (message :type "UdpMessage Structure"))
  ;[0 0 0] Events
)

(event `ConnClose`
  ;[0 0 0] Events
)

(event `Error` :!signature `self.OnError`
  (params (ErrorCode :type "ErrorCode Structure"))
  ;[0 0 0] Events
)

(event `SocketError` :!signature `self.OnSocketError`
  (params (ErrorCode :type "ErrorCode Structure"))
  ;[0 0 0] Events
)