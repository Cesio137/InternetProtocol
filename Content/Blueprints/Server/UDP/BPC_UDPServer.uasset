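; Blueprint UDP server class that lays out the socket API as an unwired scaffold, with no working logic yet.
; Empty events stand ready for listening, message, close, error and send-completion callbacks.
; Disconnected nodes show binding, sending text or buffers, closing, receive-buffer sizing and delegate assignment, none of which executes.
; Unwired AddToRoot and RemoveFromRoot calls cover protecting the object from Unreal garbage collection.
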(event `MessageSent`
  (params (ErrorCode :type "ErrorCode Structure (by ref)") (BytesSent :type Integer))
  ;[0 0 0] UDP
)

(event `BufferSent`
  (params (ErrorCode :type "ErrorCode Structure (by ref)") (BytesSent :type Integer))
  ;[0 0 0] UDP
)

(event `Listening`
  ;[0 0 0] EVENTS
)

(event `Message` :!signature `self.OnMessage`
  (params (Buffer :type "Array of Byte (by ref)") (BytesRecv :type Integer) (Endpoint :type "UdpEndpoint Structure (by ref)"))
  ;[0 0 0] EVENTS
)

(event `OnClose_Event`
  ;[0 0 0] EVENTS
)

(event `Error` :!signature `self.OnError`
  (params (ErrorCode :type "ErrorCode Structure (by ref)"))
  ;[0 0 0] EVENTS
)