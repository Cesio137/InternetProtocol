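; Blueprint WebSocket server component that lays out the server API as a node reference, with nothing wired to run.
; Unconnected nodes are grouped by host, settings, request headers, dataframe flags, messaging and connection control, alongside unused getters.
; Empty event stubs cover socket accept, transfer, message, pong, close, handshake failure, disconnect and error, but their delegate bindings never execute.
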(event `OnSocketAccepted_Event` :!signature `self.OnSocketAccepted`
  (params (Request :type "ServerRequest Structure") (Response :type "ServerResponse Structure") (Socket :type "TCPSocket Structure"))
  ;[0 0 0] EVENTS
)

(event `OnBytesTransferred_Event` :!signature `self.OnBytesTransferred`
  (params (BytesSent :type Integer) (BytesRecvd :type Integer))
  ;[0 0 0] EVENTS
)

(event `OnMessageSent_Event` :!signature `self.OnMessageSent`
  (params (HadError :type "ErrorCode Structure") (Socket :type "TCPSocket Structure"))
  ;[0 0 0] EVENTS
)

(event `OnMessageReceived_Event` :!signature `self.OnMessageReceived`
  (params (Message :type "WsMessage Structure") (Socket :type "TCPSocket Structure"))
  ;[0 0 0] EVENTS
)

(event `OnPongReceived_Event`
  ;[0 0 0] EVENTS
)

(event `OnCloseNotify_Event`
  ;[0 0 0] EVENTS
)

(event `OnClose_Event`
  ;[0 0 0] EVENTS
)

(event `OnHandshakeFail_Event` :!signature `self.OnHandshakeFail`
  (params (Response :type "ClientResponse Structure"))
  ;[0 0 0] EVENTS
)

(event `OnSocketDisconnected_Event` :!signature `self.OnSocketDisconnected`
  (params (HadError :type "ErrorCode Structure") (Socket :type "TCPSocket Structure"))
  ;[0 0 0] EVENTS
)

(event `OnError_Event` :!signature `self.OnError`
  (params (ErrorCode :type "ErrorCode Structure"))
  ;[0 0 0] EVENTS
)