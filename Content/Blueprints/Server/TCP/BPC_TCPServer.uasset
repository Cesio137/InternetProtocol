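; TCP server Blueprint component that lays out a socket server's API as an unwired template or reference, with no working logic.
; Empty handlers cover accept, transfer, send, receive, close, disconnect and error events, but their bind nodes never execute.
; Disconnected nodes show host setup, buffer and packet-split settings, string or buffer sending, and open, close and disconnect calls, alongside unused getters.
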(event `OnSocketAccepted_Event` :!signature `self.OnSocketAccepted`
  (params (Socket :type "TCPSocket Structure"))
  ;[0 0 0] EVENTS
)

(event `OnBytesTransferred_Event` :!signature `self.OnBytesTransferred`
  (params (BytesSent :type Integer) (BytesRecvd :type Integer))
  ;[0 0 0] EVENTS
)

(event `OnMessageSent_Event` :!signature `self.OnMessageSent`
  (params (HadError :type "ErrorCode Structure") (Socket :type "TCPSocket Structure"))
  ;[0 0 0] EVENTS
)

(event `OnMessageReceived_Event` :!signature `self.OnMessageReceived`
  (params (Message :type "TcpMessage Structure (by ref)") (Socket :type "TCPSocket Structure (by ref)"))
  ;[0 0 0] EVENTS
)

(event `OnClose_Event`
  ;[0 0 0] EVENTS
)

(event `OnSocketDisconnected_Event` :!signature `self.OnSocketDisconnected`
  (params (HadError :type "ErrorCode Structure") (Socket :type "TCPSocket Structure"))
  ;[0 0 0] EVENTS
)

(event `OnError_Event` :!signature `self.OnError`
  (params (ErrorCode :type "ErrorCode Structure"))
  ;[0 0 0] EVENTS
)