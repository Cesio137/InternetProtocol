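; BPC_WebsocketClient is a WebSocket client Blueprint laid out as an unwired showcase of the client's API.
; Its nodes are grouped into host, settings, handshake, dataframe, message and connection calls, plus getters, none connected to execution.
; Bind nodes pair each connection, transfer, message, pong, close and error delegate with an empty event, but never run, so the graph does nothing as it stands.
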(event `OnConnected_Event` :!signature `self.OnConnected`
  (params (Response :type "ClientResponse Structure"))
  ;[0 0 0] Events
)

(event `OnBytesTransferred_Event` :!signature `self.OnBytesTransferred`
  (params (BytesSent :type Integer) (BytesRecvd :type Integer))
  ;[0 0 0] Events
)

(event `OnMessageSent_Event` :!signature `self.OnMessageSent`
  (params (HadError :type "ErrorCode Structure"))
  ;[0 0 0] Events
)

(event `OnMessageReceived_Event` :!signature `self.OnMessageReceived`
  (params (Message :type "WsMessage Structure"))
  ;[0 0 0] Events
)

(event `OnPongReceived_Event`
  ;[0 0 0] Events
)

(event `OnCloseNotify_Event`
  ;[0 0 0] Events
)

(event `OnClose_Event`
  ;[0 0 0] Events
)

(event `OnHandshakeFail_Event` :!signature `self.OnHandshakeFail`
  (params (Response :type "ClientResponse Structure"))
  ;[0 0 0] Events
)

(event `OnError_Event` :!signature `self.OnError`
  (params (ErrorCode :type "ErrorCode Structure"))
  ;[0 0 0] Events
)