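; BPC_HttpClient is a reference Blueprint that lays out the API of an HTTP client.
; Unwired nodes cover host and request setup, sync or async payload preparation, request processing, closing and memory clearing, alongside unused getters.
; Delegate bindings point to empty handlers for payload completion, progress, response, failure, close and error.
; Nothing executes, so the graph serves as a node catalog rather than working request logic.
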(event `OnAsyncPayloadFinished_Event`
  ;[0 0 0] Events
)

(event `OnRequestProgress_Event` :!signature `self.OnRequestProgress`
  (params (BytesSent :type Integer) (BytesRecvd :type Integer))
  ;[0 0 0] Events
)

(event `OnRequestCompleted_Event` :!signature `self.OnRequestCompleted`
  (params (Response :type "ClientResponse Structure"))
  ;[0 0 0] Events
)

(event `OnRequestFail_Event` :!signature `self.OnRequestFail`
  (params (Response :type "ClientResponse Structure"))
  ;[0 0 0] Events
)

(event `OnClose_Event`
  ;[0 0 0] Events
)

(event `OnError_Event` :!signature `self.OnError`
  (params (ErrorCode :type "ErrorCode Structure"))
  ;[0 0 0] Events
)