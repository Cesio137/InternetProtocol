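; Blueprint WebSocket client component laid out as an API reference, with no executable logic wired.
; Unconnected node samples cover connection, remote host, messaging, dataframe flags, timeout and buffer settings, and handshake fields.
; Empty custom events match the delegates for connect, retry, send, receive, pong, close and error, but their bind nodes never run.
; Unused getter nodes show the available state, address and error queries.
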(event `Connected`
  ;[0 0 0] Events
)

(event `ConnectionWillRetry` :!signature `self.OnConnectionWillRetry`
  (params (attemps :type Integer))
  ;[0 0 0] Events
)

(event `MessageSent` :!signature `self.OnMessageSent`
  (params (bytesSent :type Integer))
  ;[0 0 0] Events
)

(event `MessageReceived` :!signature `self.OnMessageReceived`
  (params (message :type "WsMessage Structure"))
  ;[0 0 0] Events
)

(event `PongReceived`
  ;[0 0 0] Events
)

(event `Close_Event`
  ;[0 0 0] Events
)

(event `CloseNotify`
  ;[0 0 0] Events
)

(event `Error` :!signature `self.OnError`
  (params (code :type Integer) (exception :type String))
  ;[0 0 0] Events
)