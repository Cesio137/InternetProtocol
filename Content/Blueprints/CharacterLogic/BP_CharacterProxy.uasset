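; BP_CharacterProxy is a networked character that serves as either the locally controlled player or a stand-in for a remote one.
; When player-controlled, it handles movement and yaw input and each tick sends position and yaw as a JSON message over UDP through the GameInstance's messenger.
; Otherwise it uses Walking mode and interpolates toward RepData each tick.
; Replication is custom through InternetProtocolSubsystem, with fixed height offsets on send and receive.
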(event `self.ReceiveBeginPlay`
  (bind _returnvalue (`InternetProtocolSubsystem.CreateJsonObject` (subsystem `InternetProtocolSubsystem`)))
  (bind _output_get (set `self.RepJson` _returnvalue))
  (`JavaScriptObjectNotation.ConstructJson` _output_get
    (:`Success`
      (`JavaScriptObjectNotation.SetStringField` (`self.RepJson`) "event" "message_order")
      (`JavaScriptObjectNotation.SetIntegerField` (`self.RepJson`) "ID" 0)
      (`JavaScriptObjectNotation.SetIntegerField` (`self.RepJson`) "condition" 2)
      (if (not (`self.IsPlayerControlled`))
        (`CharacterMovementComponent.SetMovementMode` (`self.CharacterMovement`) "MOVE_Walking" 0)))))

(event `self.ReceiveTick`
  (params (DeltaSeconds :type "Float (single-precision)"))
  (if (`self.IsPlayerControlled`)
    (`self.ReplicateTransform`)
    (else
      (`self.UpdateTransform`))))

(event `InputAxis|MoveForward`
  (params (AxisValue :type "Float (single-precision)"))
  (`self.AddMovementInput` (`self.GetActorForwardVector`) AxisValue))

(event `InputAxis|MoveRight`
  (params (AxisValue :type "Float (single-precision)"))
  (`self.AddMovementInput` (`self.GetActorRightVector`) AxisValue))

(event `InputAxis|LookRight`
  (params (AxisValue :type "Float (single-precision)"))
  (`self.AddControllerYawInput` AxisValue))

(fn `ReplicateTransform`
  (bind (_returnvalue_x _returnvalue_y _returnvalue_z) (`KismetMathLibrary.BreakVector` (`self.K2_GetActorLocation`)))
  (bind (_returnvalue_roll _returnvalue_pitch _returnvalue_yaw) (`KismetMathLibrary.BreakRotator` (`self.K2_GetActorRotation`)))
  (bind _returnvalue_x_2 (`KismetMathLibrary.BreakVector` (`self.K2_GetActorLocation`)))
  (bind (_returnvalue_x_3 _returnvalue_y_2) (`KismetMathLibrary.BreakVector` (`self.K2_GetActorLocation`)))
  (`/Engine/EditorBlueprintResources/StandardMacros.IsValid` (`self.RepJson`)
    (:`Is Valid`
      (`JavaScriptObjectNotation.SetFloatField` (`self.RepJson`) "positionX" _returnvalue_x_2)
      (`JavaScriptObjectNotation.SetFloatField` (`self.RepJson`) "positionY" _returnvalue_y_2)
      (`JavaScriptObjectNotation.SetFloatField` (`self.RepJson`) "positionZ" (+ _returnvalue_z 45.0))
      (`JavaScriptObjectNotation.SetFloatField` (`self.RepJson`) "rotationZ" _returnvalue_yaw)
      (bind _return (message `/Game/Blueprints/Interfaces/BPI_Gameinstance.Get` (`GameplayStatics.GetGameInstance`)))
      (`UDPClient.send` (`/Game/Blueprints/Game/BP_Gameinstance.UDP` _return) (`JavaScriptObjectNotation.ToString` (`self.RepJson`))))))

(fn `UpdateTransform`
  (locals (Location :type "Vector Structure") (InterpLocation :type "Vector Structure") (Rotation :type "Rotator Structure") (InterpRotation :type "Rotator Structure" :default (struct)))
  (bind (_repdata_id _repdata_positionx _repdata_positiony _repdata_positionz _repdata_rotationz) (break `/Game/Blueprints/Data/FMessageOrder` (`self.RepData`)))
  (bind (_repdata_id_2 _repdata_positionx_2 _repdata_positiony_2 _repdata_positionz_2) (break `/Game/Blueprints/Data/FMessageOrder` (`self.RepData`)))
  (bind _output_get (set `local.Location` (`KismetMathLibrary.MakeVector` _repdata_positionx_2 _repdata_positiony_2 (+ _repdata_positionz_2 112.0))))
  (bind _output_get_2 (set `local.InterpLocation` (`KismetMathLibrary.VInterpTo` (`self.K2_GetActorLocation`) _output_get (`GameplayStatics.GetWorldDeltaSeconds`) 30.0)))
  (`self.K2_SetActorLocation` _output_get_2 false true)
  (bind _output_get_3 (set `local.Rotation` (`KismetMathLibrary.MakeRotator` 0.0 0.0 _repdata_rotationz)))
  (bind _output_get_4 (set `local.InterpRotation` (`KismetMathLibrary.RInterpTo` (`self.K2_GetActorRotation`) _output_get_3 (`GameplayStatics.GetWorldDeltaSeconds`) 30.0)))
  (`self.K2_SetActorRotation` _output_get_4))

(fn `UserConstructionScript`)